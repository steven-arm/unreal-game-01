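; BP_Destructible is a breakable prop built from a Geometry Collection and a Box trigger.
; It breaks once, either when a BP_Master_Hitbox_01 overlaps the Box or on any component hit; the hitbox's damage is only printed.
; Breaking enables physics with mass scaled by Box size, then disables Box collision after a short delay and later destroys the actor.
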(event OnComponentBeginOverlap(Box)
  (params (OverlappedComponent :type Primitive%20Component%20Object%20Reference) (OtherActor :type Actor%20Object%20Reference) (OtherComp :type Primitive%20Component%20Object%20Reference) (OtherBodyIndex :type Integer) (bFromSweep :type Boolean) (SweepResult :type Hit%20Result%20Structure%20%28by%20ref%29))
  (bind _box (Variables|Default|GetBox))
  (bind _returnvalue (Transformation|GetWorldScale _box))
  (bind _returnvalue_2 (Math|Vector|VectorLength _returnvalue))
  (bind _asbp_master_hitbox_01 (Utilities|Casting|CastToBP_Master_Hitbox_01 OtherActor))
  (Development|PrintString (Utilities|String|ToString(Float) (Variables|/Game/Blueprints/Hitbox/BP_Master_Hitbox_01.BP_Master_Hitbox_01_C|GetDamage%20of%20Ability _asbp_master_hitbox_01)))
  (if (not (Variables|Default|GetIsHit))
    (Variables|Default|SetIsHit true)
    (Physics|SetSimulatePhysics (Variables|Default|GetGeometryCollection) true)
    (Class|PrimitiveComponent|SetMassScale (Variables|Default|GetGeometryCollection) "None" (* _returnvalue_2 1e+01))
    (Development|PrintString (Utilities|String|ToString(Float) _returnvalue_2))
    (Utilities|FlowControl|Delay 0.2)
    (Collision|SetCollisionEnabled (Variables|Default|GetBox) "NoCollision")
    (Utilities|FlowControl|Delay 4.0)
    (Actor|DestroyActor)))

(event OnComponentHit(Box)
  (params (HitComponent :type Primitive%20Component%20Object%20Reference) (OtherActor :type Actor%20Object%20Reference) (OtherComp :type Primitive%20Component%20Object%20Reference) (NormalImpulse :type Vector :default "0, 0, 0") (Hit :type Hit%20Result%20Structure%20%28by%20ref%29))
  (bind _box (Variables|Default|GetBox))
  (bind _returnvalue (Transformation|GetWorldScale _box))
  (bind _returnvalue_2 (Math|Vector|VectorLength _returnvalue))
  (if (not (Variables|Default|GetIsHit))
    (Variables|Default|SetIsHit true)
    (Physics|SetSimulatePhysics (Variables|Default|GetGeometryCollection) true)
    (Class|PrimitiveComponent|SetMassScale (Variables|Default|GetGeometryCollection) "None" (* _returnvalue_2 1e+01))
    (Development|PrintString (Utilities|String|ToString(Float) _returnvalue_2))
    (Utilities|FlowControl|Delay 0.2)
    (Collision|SetCollisionEnabled (Variables|Default|GetBox) "NoCollision")
    (Utilities|FlowControl|Delay 4.0)
    (Actor|DestroyActor)))

(event EventBeginPlay)

(event Collision|EventActorBeginOverlap
  (params (OtherActor :type Actor%20Object%20Reference)))

(event EventTick
  (params (DeltaSeconds :type Float%20%28single-precision%29)))

(fn ConstructionScript)