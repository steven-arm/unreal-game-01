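; Game mode that owns the Dawn player HUD and acts as the relay for gameplay updates to it.
; On BeginPlay it creates the UI_Dawn_01 widget, adds it to the viewport and seeds the ammo display from BP_Dawn's MaxAmmo, cast from player controller 0.
; Its custom events forward ammo, reload, secondary and ultimate cooldown, percent and boss-fight updates straight to the widget's matching functions.
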(event Custom|Change%20Ammo
  (params (Ammo :type Integer))
  (Default|UpdateAmmo (stale EventBeginPlay _returnvalue) Ammo))

(event Custom|Reloading
  (params (Reload%20Time :type Float%20%28double-precision%29))
  (Default|Reloading (stale EventBeginPlay _returnvalue) Reload%20Time))

(event Custom|Secondary%20Cooldown
  (params (Cooldown :type Float%20%28double-precision%29))
  (Default|SecondaryCooldown (stale EventBeginPlay _returnvalue) Cooldown))

(event Custom|Ult%20Cooldown
  (params (Cooldown :type Float%20%28double-precision%29))
  (Default|UltCooldown (stale EventBeginPlay _returnvalue) Cooldown))

(event Custom|Set%20Percent
  (params (Percent :type Float%20%28double-precision%29))
  (Default|SetPercent (stale EventBeginPlay _returnvalue) Percent))

(event Custom|Start%20Boss%20Fight
  (params (Boss%20Name :type String))
  (Default|StartBossFight (stale EventBeginPlay _returnvalue) Boss%20Name))

(event Custom|Set%20Boss%20Percent
  (params (Percent :type Float%20%28double-precision%29))
  (Default|SetBossPercent (stale EventBeginPlay _returnvalue) Percent))

(event EventBeginPlay
  (bind _returnvalue (UserInterface|CreateWidget "/Game/Blueprints/UI/UI_Dawn_01.UI_Dawn_01_C"))
  (UserInterface|Viewport|AddtoViewport _returnvalue 0)
  (bind _asbp_dawn (Utilities|Casting|CastToBP_Dawn (Game|GetPlayerController 0)))
  (Default|UpdateAmmo _returnvalue (Variables|/Game/Blueprints/Character/Dawn/Controls/BP_Dawn.BP_Dawn_C|GetMaxAmmo _asbp_dawn)))

(event EventTick
  (params (DeltaSeconds :type Float%20%28single-precision%29)))

(fn ConstructionScript)