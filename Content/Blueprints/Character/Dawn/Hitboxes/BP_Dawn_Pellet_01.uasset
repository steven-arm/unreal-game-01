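; BP_Dawn_Pellet_01 is a pellet hitbox for the Dawn character that delivers damage on impact.
; On spawn it attaches a Niagara effect to its sphere and destroys itself after ten seconds.
; The first sphere hit spawns a BP_Dawn_Pellet_Hit_01 at the impact point, then destroys the pellet.
; Damage passed to that actor falls off inversely with flight time; Crit is forwarded, but both its damage branches are identical.
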(event OnComponentHit(Sphere)
  (params (HitComponent :type Primitive%20Component%20Object%20Reference) (OtherActor :type Actor%20Object%20Reference) (OtherComp :type Primitive%20Component%20Object%20Reference) (NormalImpulse :type Vector :default "0, 0, 0") (Hit :type Hit%20Result%20Structure%20%28by%20ref%29))
  (bind _returnvalue (Actor|GetGameTimeSinceCreation))
  (bind _damage (Variables|Default|GetDamage))
  (bind _crit (Variables|Default|GetCrit))
  (bind _returnvalue_2 (Math|Float|Clamp(Float) _returnvalue 0.01))
  (bind _returnvalue_3 (* _returnvalue_2 1e+02))
  (bind _returnvalue_4 (/ 1.0 _returnvalue_3))
  (bind _returnvalue_5 (* _damage _returnvalue_4))
  (Utilities|FlowControl|DoOnce false
    (:Completed
      (Game|SpawnActorfromClass "/Game/Blueprints/Character/Dawn/Hitboxes/BP_Dawn_Pellet_Hit_01.BP_Dawn_Pellet_Hit_01_C" (Math|Conversions|ToTransform(Vector) (.Location (Collision|BreakHitResult Hit))) "Undefined" "MultiplyWithRoot" 0 0.0 (Math|Float|SelectFloat _returnvalue_5 _returnvalue_5 _crit) _crit 0)
      (Actor|DestroyActor))))

(event EventBeginPlay
  (Niagara|SpawnSystemAttached "/Game/Blueprints/Niagara/NS_test_01.NS_test_01" (Variables|Default|GetSphere) "None" "0, 0, 0" "0, 0, 0" "KeepRelativeOffset" false)
  (Utilities|FlowControl|Delay 1e+01)
  (Actor|DestroyActor))

(event Collision|EventActorBeginOverlap
  (params (OtherActor :type Actor%20Object%20Reference)))

(event EventTick
  (params (DeltaSeconds :type Float%20%28single-precision%29)))

(fn ConstructionScript)