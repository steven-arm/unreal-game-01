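; Short-lived parry hitbox that destroys incoming BP_Master_Hitbox_01 attack hitboxes overlapping its box.
; The box collides only for a brief window after spawn, and the actor destroys itself a few seconds later.
; The first successful overlap briefly sets Parried on the BP_Dawn instigator and plays its parry VFX.
; A DoOnce limits that response to once per instance, while later overlapping hitboxes are still destroyed.
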(event OnComponentBeginOverlap(Box)
  (params (OverlappedComponent :type Primitive%20Component%20Object%20Reference) (OtherActor :type Actor%20Object%20Reference) (OtherComp :type Primitive%20Component%20Object%20Reference) (OtherBodyIndex :type Integer) (bFromSweep :type Boolean) (SweepResult :type Hit%20Result%20Structure%20%28by%20ref%29))
  (Utilities|Casting|CastToBP_Master_Hitbox_01 OtherActor)
  (Utilities|IsValid OtherActor
    (:Is%20Valid
      (Actor|DestroyActor OtherActor))
    (:Is%20Not%20Valid
      _))
  (Utilities|FlowControl|DoOnce false
    (:Completed
      (bind _asbp_dawn (Utilities|Casting|CastToBP_Dawn (Game|GetInstigator)))
      (Variables|/Game/Blueprints/Character/Dawn/Controls/BP_Dawn.BP_Dawn_C|SetParried _asbp_dawn true)
      (Default|ParryVFX _asbp_dawn)
      (Utilities|FlowControl|Delay 0.2)
      (Variables|/Game/Blueprints/Character/Dawn/Controls/BP_Dawn.BP_Dawn_C|SetParried _asbp_dawn false))))

(event EventBeginPlay
  (|CallParentFunction)
  (Utilities|FlowControl|Delay 0.2)
  (Collision|SetCollisionEnabled (Variables|Default|GetBox) "NoCollision")
  (Utilities|FlowControl|Delay 4.0)
  (Actor|DestroyActor))

(event Collision|EventActorBeginOverlap
  (params (OtherActor :type Actor%20Object%20Reference))
  (|CallParentFunction OtherActor) ; This node is disabled and will not be called.\nDrag off pins to build functionality.
)

(event EventTick
  (params (DeltaSeconds :type Float%20%28single-precision%29))
  (|CallParentFunction DeltaSeconds) ; This node is disabled and will not be called.\nDrag off pins to build functionality.
)

(fn ConstructionScript
  (|CallParentFunction))