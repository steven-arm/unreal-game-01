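; BP_Master_Enemy_01 is a master enemy Blueprint that handles taking damage and dying.
; AnyDamage responds only to BP_Master_Hitbox_01 causers, reducing Health and spawning a damage number carrying the hitbox's Crit value.
; A helper places that number above the actor using the mesh bounds' vertical extent.
; When Health runs out, small enemies enable mesh physics simulation, and all are destroyed after a short delay.
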(event EventBeginPlay)

(event Collision|EventActorBeginOverlap
  (params (OtherActor :type Actor%20Object%20Reference)))

(event EventTick
  (params (DeltaSeconds :type Float%20%28single-precision%29)))

(event Game|Damage|EventAnyDamage
  (params (Damage :type Float%20%28single-precision%29) (DamageType :type Damage%20Type%20Object%20Reference) (InstigatedBy :type Controller%20Object%20Reference) (DamageCauser :type Actor%20Object%20Reference))
  (bind _asbp_master_hitbox_01 (Utilities|Casting|CastToBP_Master_Hitbox_01 DamageCauser))
  (bind _world_transform (CallFunction|GetTopOfBoundingBox))
  (Game|SpawnActorfromClass "/Game/Blueprints/UI/BP_Damage_Number_01.BP_Damage_Number_01_C" _world_transform "Undefined" "MultiplyWithRoot" 0 "0.000000" (Variables|/Game/Blueprints/Hitbox/BP_Master_Hitbox_01.BP_Master_Hitbox_01_C|GetCrit _asbp_master_hitbox_01) 0)
  (bind _output_get (Variables|Default|SetHealth (- (Variables|Default|GetHealth) Damage)))
  (if (<= _output_get 0.0)
    (if (< (Variables|Default|GetSize) 2)
      (Physics|SetSimulatePhysics (Variables|Default|Getmesh) true))
    (Utilities|FlowControl|Delay 3.0)
    (Actor|DestroyActor)))

(fn ConstructionScript)

(fn GetTopOfBoundingBox
  (bind _returnvalue (Transformation|GetActorLocation))
  (bind (_x _y _z) (Math|Vector|BreakVector _returnvalue))
  (return (Math|Transform|MakeTransform (Math|Vector|MakeVector _x _y (+ _z (.Z (Math|Vector|BreakVector (.BoxExtent (Collision|GetComponentBounds (Variables|Default|Getmesh))))))))))