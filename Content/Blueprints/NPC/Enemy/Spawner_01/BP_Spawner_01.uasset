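; BP_Spawner_01 is the "Insect Spawner", a damageable enemy that keeps producing spiders while it has health.
; On BeginPlay it sets up its named healthbar widget, which is made visible the first time it takes damage.
; A self-recalling Spawn event waits a random delay, then randomly spawns one of two spider classes with a controller at a reachable point ahead.
; The loop ends when health runs out or a spawn fails.
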(event Custom|Spawn
  (bind _returnvalue (Transformation|GetActorForwardVector))
  (bind _returnvalue_2 (Transformation|GetActorLocation))
  (bind _returnvalue_3 (* _returnvalue 5e+02))
  (bind _returnvalue_4 (+ _returnvalue_2 _returnvalue_3))
  (bind _randomlocation (AI|Navigation|GetRandomReachablePointinRadius _returnvalue_4 2e+03 0 0))
  (Utilities|FlowControl|Delay (Math|Random|RandomFloatinRange 5.0 1e+01))
  (if (> (Variables|Default|GetHealth) 0.0)
    (Utilities|FlowControl|MultiGate true true -1
      (:Out%200
        (bind _returnvalue_5 (Game|SpawnActorfromClass "/Game/Blueprints/NPC/Enemy/Spider_01/BP_Spider01.BP_Spider01_C" (Math|Transform|MakeTransform _randomlocation "0, 0, 0" "1.000000,1.000000,1.000000") "Undefined" "MultiplyWithRoot" 0 0))
        (Utilities|IsValid _returnvalue_5
          (:Is%20Valid
            (Pawn|SpawnDefaultController _returnvalue_5))))
      (:Out%201
        (bind _returnvalue_6 (Game|SpawnActorfromClass "/Game/Blueprints/NPC/Enemy/Spider_02/BP_Spider02.BP_Spider02_C" (Math|Transform|MakeTransform _randomlocation "0, 0, 0" "1.000000,1.000000,1.000000") "Undefined" "MultiplyWithRoot" 0 0))
        (Utilities|IsValid _returnvalue_6
          (:Is%20Valid
            (Pawn|SpawnDefaultController _returnvalue_6)))))
    (CallFunction|Spawn)))

(event Custom|OnTakeAnyDamage_Event
  (params (DamagedActor :type Actor%20Object%20Reference) (Damage :type Float%20%28single-precision%29) (DamageType :type Damage%20Type%20Object%20Reference) (InstigatedBy :type Controller%20Object%20Reference) (DamageCauser :type Actor%20Object%20Reference))
  (Utilities|FlowControl|DoOnce false
    (:Completed
      (Rendering|SetVisibility (Variables|Default|GetHealthbar) true false))))

(event EventBeginPlay
  (|CallParentFunction)
  (Variables|Default|SetSize 1)
  (bind _output_get (Variables|Default|SetHealth 1e+03))
  (Variables|Default|SetMax%20Health _output_get)
  (bind _output_get_2 (Variables|Default|SetDisplay%20Name "Insect Spawner"))
  (bind _aswbp_enemy_healthbar_01 (Utilities|Casting|CastToWBP_Enemy_Healthbar_01 (UserInterface|GetWidget (Variables|Default|GetHealthbar))))
  (Default|SetName _aswbp_enemy_healthbar_01 _output_get_2)
  (Default|SetPercent _aswbp_enemy_healthbar_01 1.0)
  (EventDispatchers|BindEventtoOnTakeAnyDamage (delegate Custom|OnTakeAnyDamage_Event))
  (Utilities|FlowControl|Delay 0.2)
  (CallFunction|Spawn))

(event Collision|EventActorBeginOverlap
  (params (OtherActor :type Actor%20Object%20Reference))
  (|CallParentFunction OtherActor) ; This node is disabled and will not be called.\nDrag off pins to build functionality.
)

(event EventTick
  (params (DeltaSeconds :type Float%20%28single-precision%29))
  (|CallParentFunction DeltaSeconds) ; This node is disabled and will not be called.\nDrag off pins to build functionality.
)

(fn ConstructionScript
  (|CallParentFunction))