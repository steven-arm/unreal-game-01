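; Phase 2 Brood Mother boss, shown as "Cursed Husk Warrior", that sets its health and size and runs an intro cutscene when its fight starts.
; The cutscene finds three numbered location markers, spawns a Mother Husk and teleports the player.
; It hides the UI and locks input while the level's first-found sequence plays, then restores both.
; The game mode receives the boss name and a full health bar.
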(event Custom|Initial%20Cutscene
  (bind _returnvalue (Game|GetPlayerController 0))
  (bind _outactors (Actor|GetAllActorsOfClass "/Game/Blueprints/World/BP_Location_Set.BP_Location_Set_C"))
  (for _array_element _outactors
    (if (== (Variables|/Game/Blueprints/World/BP_Location_Set.BP_Location_Set_C|GetPoint%20Number _array_element) 0)
      (Variables|Default|SetTarget%201 (Transformation|GetActorLocation _array_element))
      (elif (== (Variables|/Game/Blueprints/World/BP_Location_Set.BP_Location_Set_C|GetPoint%20Number _array_element) 1)
        (Variables|Default|SetTarget%202 (Transformation|GetActorLocation _array_element))
        (elif (== (Variables|/Game/Blueprints/World/BP_Location_Set.BP_Location_Set_C|GetPoint%20Number _array_element) 2)
          (Variables|Default|SetTarget%203 (Transformation|GetActorLocation _array_element))))))
  (Game|SpawnActorfromClass "/Game/Blueprints/NPC/Enemy/Brood_Mother_01/BP_Mother_Husk_01.BP_Mother_Husk_01_C" (Math|Transform|MakeTransform (Variables|Default|GetTarget%203) (Math|Rotator|FindLookatRotation (Variables|Default|GetTarget%202) (Variables|Default|GetTarget%201)) "1.000000,1.000000,1.000000") "Undefined" "MultiplyWithRoot" 0 0)
  (bind _asbp_gamemode_0 (Utilities|Casting|CastToBP_Gamemode_0 (Game|GetGameMode)))
  (Default|ToggleUI _asbp_gamemode_0)
  (Transformation|SetActorLocation (Variables|Default|GetPlayer%20Character) (Variables|Default|GetTarget%201) false false)
  (Pawn|SetControlRotation _returnvalue (Math|Rotator|FindLookatRotation (Variables|Default|GetTarget%202) (Variables|Default|GetTarget%201)))
  (Input|DisableInput (Variables|Default|GetPlayer%20Character) _returnvalue)
  (bind _returnvalue_2 (Actor|GetActorOfClass "/Script/LevelSequence.LevelSequenceActor"))
  (Sequencer|Player|Play (Variables|/Script/LevelSequence.LevelSequenceActor|GetSequencePlayer _returnvalue_2) :!class /Script/MovieScene.MovieSceneSequencePlayer)
  (Utilities|FlowControl|Delay (Class|TimeManagementBlueprintLibrary|ToSeconds(QualifiedFrameTime) (Media|MediaPlayer|GetDuration (Variables|/Script/LevelSequence.LevelSequenceActor|GetSequencePlayer _returnvalue_2))))
  (Pawn|SetControlRotation _returnvalue (Math|Rotator|FindLookatRotation (Variables|Default|GetTarget%201) (Variables|Default|GetTarget%202)))
  (Input|EnableInput (Variables|Default|GetPlayer%20Character) 0)
  (bind _asbp_gamemode_0_2 (Utilities|Casting|CastToBP_Gamemode_0 (Game|GetGameMode)))
  (Default|ToggleUI _asbp_gamemode_0_2))

(event EventBeginPlay
  (|CallParentFunction)
  (Variables|Default|SetSize 10)
  (bind _output_get (Variables|Default|SetHealth 5e+03))
  (Variables|Default|SetMax%20Health _output_get)
  (bind _output_get_2 (Variables|Default|SetDisplay%20Name "Cursed Husk Warrior"))
  (Variables|Default|SetPlayer%20Character (Game|GetPlayerCharacter 0)))

(event Collision|EventActorBeginOverlap
  (params (OtherActor :type Actor%20Object%20Reference))
  (|CallParentFunction OtherActor) ; This node is disabled and will not be called.\nDrag off pins to build functionality.
)

(event EventTick
  (params (DeltaSeconds :type Float%20%28single-precision%29))
  (|CallParentFunction DeltaSeconds) ; This node is disabled and will not be called.\nDrag off pins to build functionality.
)

(event EventStartBossFight
  (|CallParentFunction)
  (CallFunction|InitialCutscene)
  (bind _asbp_gamemode_0 (Utilities|Casting|CastToBP_Gamemode_0 (Game|GetGameMode)))
  (Default|StartBossFight _asbp_gamemode_0 (stale EventBeginPlay _output_get_2))
  (Default|SetBossPercent _asbp_gamemode_0 1.0)
  (Utilities|FlowControl|Delay 2.0))

(fn ConstructionScript
  (|CallParentFunction))