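; Insect Brood Mother boss Blueprint that opens its fight with a leap toward the player and a slam, registering with the game mode.
; A random MultiGate picks charge, slam, forward strike, long-range spit or walk, each looping back to StartAttack while health remains.
; Attacks combine AI movement and animation overrides with timed hitbox or projectile spawns, most adding camera shake.
; NextPhase uses BP_Location_Set markers to spawn and start the Husk Knight.
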(event Custom|Attack:%20Charge
  (bind (_origin _boxextent) (Collision|GetActorBounds false false))
  (bind _self self)
  (bind _charactermovement (Variables|Character|GetCharacterMovement))
  (bind _player_character (Variables|Default|GetPlayer%20Character))
  (bind _returnvalue (Class|CharacterMovementComponent|GetLastUpdateLocation _charactermovement))
  (bind _returnvalue_2 (Transformation|GetActorLocation _player_character))
  (bind _returnvalue_3 (Transformation|GetActorTransform _self))
  (bind _returnvalue_4 (Math|Rotator|FindLookatRotation _returnvalue _returnvalue_2))
  (Transformation|SetActorRotation (Math|Rotator|MakeRotator (.roll _returnvalue_4) (.pitch (Transformation|GetActorRotation _player_character)) (.yaw _returnvalue_4)))
  (Variables|Default|SetCharge%20Start%20Location _returnvalue)
  (Variables|Default|SetCharge%20End%20Location (Transformation|GetActorLocation (Game|Player|GetPlayerPawn 0)))
  (Components|Animation|OverrideAnimationData (Variables|Character|GetMesh) "/Game/Blueprints/NPC/Enemy/Brood_Mother_01/Phase_1/Animations/AS_BroodMother_Walk_01.AS_BroodMother_Walk_01" true true 0.0 2.0)
  (Collision|SetCollisionResponsetoChannel (Variables|Default|GetCapsuleComponent) "ECC_Pawn" "ECR_Ignore")
  (bind _location (Timeline|Charge PlayFromStart)
    (:Update
      (AI|AIMoveTo self "0, 0, 0" (Variables|Default|GetPlayer%20Character) 1e+03 false))
    (:Finished
      (Components|Animation|SetAnimationMode (Variables|Character|GetMesh) "AnimationBlueprint" true)
      (Collision|SetCollisionResponsetoChannel (Variables|Default|GetCapsuleComponent) "ECC_Pawn" "ECR_Block")
      (CallFunction|StartAttack))
    (:Create%20Hitbox
      (Game|SpawnActorfromClass "/Game/Blueprints/NPC/Enemy/Brood_Mother_01/Phase_1/Hitboxes/BP_BroodMother_Charge_01.BP_BroodMother_Charge_01_C" (Math|Transform|MakeTransform (Math|Vector|MakeVector (.x _origin) (.y _origin) (- (.z _origin) (.z _boxextent))) (.rotation _returnvalue_3) (.scale _returnvalue_3)) "Undefined" "MultiplyWithRoot" 0 1e+02 false 0)
      (CallFunction|CameraShake))))

(event Custom|Attack:%20Slam
  (bind _returnvalue (Transformation|GetActorTransform))
  (bind (_origin _boxextent) (Collision|GetActorBounds false false))
  (bind _mesh (Variables|Character|GetMesh))
  (bind _returnvalue_2 (- (.z _origin) (.z _boxextent)))
  (bind _returnvalue_3 (Math|Vector|MakeVector (.x _origin) (.y _origin) _returnvalue_2))
  (AI|AIMoveTo self "0, 0, 0" (Variables|Default|GetPlayer%20Character) 1.5e+03 false
    (:OnSuccess
      _)
    (:OnFail
      _))
  (Components|Animation|OverrideAnimationData _mesh "/Game/Blueprints/NPC/Enemy/Brood_Mother_01/Phase_1/Animations/AS_BroodMother_Slam_01.AS_BroodMother_Slam_01" false true 0.0 1.0)
  (Utilities|FlowControl|Delay 1.5)
  (Game|SpawnActorfromClass "/Game/Blueprints/NPC/Enemy/Brood_Mother_01/Phase_1/Hitboxes/BP_BroodMother_Slam_01.BP_BroodMother_Slam_01_C" (Math|Transform|MakeTransform _returnvalue_3 (.rotation _returnvalue) (.scale _returnvalue)) "Undefined" "MultiplyWithRoot" 0 6e+02 true 0)
  (Niagara|SpawnSystematLocation "/Game/Blueprints/NPC/Enemy/Brood_Mother_01/Phase_1/FX/NS_BroodMother_Slam.NS_BroodMother_Slam" _returnvalue_3 "0, 0, 0" (.scale _returnvalue))
  (CallFunction|CameraShake)
  (Utilities|FlowControl|Delay 0.5)
  (Components|Animation|SetAnimationMode _mesh "AnimationBlueprint" true)
  (CallFunction|StartAttack))

(event Custom|Attack:%20Forward
  (bind _returnvalue (Transformation|GetActorTransform))
  (bind (_origin _boxextent) (Collision|GetActorBounds false false))
  (bind _returnvalue_2 (Transformation|GetActorForwardVector))
  (bind _mesh (Variables|Character|GetMesh))
  (bind _returnvalue_3 (* _returnvalue_2 4e+02))
  (bind _returnvalue_4 (- (.z _origin) (.z _boxextent)))
  (bind _returnvalue_5 (Math|Vector|MakeVector (.x _origin) (.y _origin) _returnvalue_4))
  (bind _returnvalue_6 (+ _returnvalue_5 _returnvalue_3))
  (AI|AIMoveTo self "0, 0, 0" (Variables|Default|GetPlayer%20Character) 1.5e+03 false
    (:OnSuccess
      _)
    (:OnFail
      _))
  (Components|Animation|OverrideAnimationData _mesh "/Game/Blueprints/NPC/Enemy/Brood_Mother_01/Phase_1/Animations/AS_BroodMother_Front_01.AS_BroodMother_Front_01" false true 0.0 1.0)
  (Utilities|FlowControl|Delay 0.58)
  (Game|SpawnActorfromClass "/Game/Blueprints/NPC/Enemy/Brood_Mother_01/Phase_1/Hitboxes/BP_BroodMother_Front_01.BP_BroodMother_Front_01_C" (Math|Transform|MakeTransform _returnvalue_6 (.rotation _returnvalue) (.scale _returnvalue)) "Undefined" "MultiplyWithRoot" 0 2e+02 false 0)
  (Niagara|SpawnSystematLocation "/Game/Blueprints/NPC/Enemy/Brood_Mother_01/Phase_1/FX/NS_BroodMother_Slam.NS_BroodMother_Slam" _returnvalue_6 "0, 0, 0" (.scale _returnvalue))
  (CallFunction|CameraShake)
  (Utilities|FlowControl|Delay 0.92)
  (Components|Animation|SetAnimationMode _mesh "AnimationBlueprint" true)
  (CallFunction|StartAttack))

(event Custom|Attack:%20Spit
  (bind _player_character (Variables|Default|GetPlayer%20Character))
  (bind _mesh (Variables|Character|GetMesh))
  (bind _returnvalue (Transformation|GetSocketLocation _mesh "Tail1Socket"))
  (bind _mesh_2 (Variables|/Script/Engine.Character|GetMesh _player_character))
  (bind (_origin _boxextent) (Collision|GetComponentBounds _mesh_2))
  (CallFunction|BootLegFacePlayer)
  (if (< (Math|Vector|Distance(Vector) (Transformation|GetActorLocation (Variables|Default|GetPlayer%20Character)) (Transformation|GetActorLocation)) 4e+03)
    (CallFunction|StartAttack)
    (else
      (Components|Animation|OverrideAnimationData (Variables|Character|GetMesh) "/Game/Blueprints/NPC/Enemy/Brood_Mother_01/Phase_1/Animations/AS_BroodMother_Spit_01.AS_BroodMother_Spit_01" false true 0.0 1.0)
      (Utilities|FlowControl|Delay 1.28)
      (Game|SpawnActorfromClass "/Game/Blueprints/NPC/Enemy/Spider_02/BP_Spider_02_Projectile.BP_Spider_02_Projectile_C" (Math|Transform|MakeTransform _returnvalue (Math|Rotator|FindLookatRotation _returnvalue (Math|Vector|MakeVector (.x _origin) (.y _origin) (+ (.z _origin) (.z _boxextent)))) "10.000000,10.000000,10.000000") "Undefined" "MultiplyWithRoot" 0 25.0 false 0)
      (Utilities|FlowControl|Delay 0.64)
      (Components|Animation|SetAnimationMode (Variables|Character|GetMesh) "AnimationBlueprint" true)
      (CallFunction|StartAttack))))

(event Custom|Start%20Attack
  (Utilities|FlowControl|Delay (Math|Random|RandomFloatinRange 0.5 1.0))
  (AI|Navigation|StopMovement (Pawn|GetController))
  (if (> (Variables|Default|GetHealth) 0.0)
    (Utilities|FlowControl|MultiGate true true -1
      (:Out%200
        (CallFunction|Attack:Charge))
      (:Out%201
        (CallFunction|Attack:Slam))
      (:Out%202
        (CallFunction|Attack:Forward))
      (:Out%203
        (CallFunction|Attack:Spit))
      (:Out%204
        (CallFunction|JustWalk)))))

(event Custom|Boot%20Leg%20Face%20Player
  (bind _self self)
  (AI|AIMoveTo _self "0, 0, 0" (Variables|Default|GetPlayer%20Character) 2e+03 false
    (:then
      (Utilities|FlowControl|Delay 0.5)
      (AI|Navigation|StopMovement (Pawn|GetController _self)))))

(event Custom|Camera%20Shake
  (Game|Feedback|ClientStartCameraShake (Game|GetPlayerController 0) "/Game/Blueprints/Character/Dawn/FX/BP_Camera_Shake_01.BP_Camera_Shake_01_C" (* (- 1.0 (/ (Math|Float|Clamp(Float) (Math|Vector|Distance(Vector) (Transformation|GetWorldLocation (Variables|Character|GetMesh)) (Transformation|GetActorLocation (Variables|Default|GetPlayer%20Character))) 0.0 3e+03) 3e+03)) (* (Math|Random|RandomFloatinRange 0.7 1.3) 2.0)) "CameraLocal" "0, 0, 0"))

(event Custom|Just%20Walk
  (AI|AIMoveTo self "0, 0, 0" (Variables|Default|GetPlayer%20Character) 2e+03 false
    (:OnSuccess
      _)
    (:OnFail
      _))
  (CallFunction|StartAttack))

(event EventBeginPlay
  (|CallParentFunction)
  (Variables|Default|SetSize 10)
  (bind _output_get (Variables|Default|SetHealth 5e+03))
  (Variables|Default|SetMax%20Health _output_get)
  (Variables|Default|SetDisplay%20Name "Insect Brood Mother")
  (Variables|Default|SetPhases 2)
  (Variables|Default|SetPlayer%20Character (Game|GetPlayerCharacter 0)))

(event Collision|EventActorBeginOverlap
  (params (OtherActor :type Actor%20Object%20Reference))
  (|CallParentFunction OtherActor) ; This node is disabled and will not be called.\nDrag off pins to build functionality.
)

(event EventTick
  (params (DeltaSeconds :type Float%20%28single-precision%29))
  (|CallParentFunction DeltaSeconds) ; This node is disabled and will not be called.\nDrag off pins to build functionality.
)

(event EventStartBossFight
  (bind _returnvalue (Game|Player|GetPlayerPawn 0))
  (bind _returnvalue_2 (Transformation|GetActorTransform))
  (bind (_origin _boxextent) (Collision|GetActorBounds false false))
  (bind _returnvalue_3 (Transformation|GetActorLocation))
  (bind _returnvalue_4 (Transformation|GetActorLocation _returnvalue))
  (bind _returnvalue_5 (- (.z _origin) (.z _boxextent)))
  (bind _returnvalue_6 (Math|Vector|GetUnitDirection(Vector) _returnvalue_3 _returnvalue_4))
  (bind _returnvalue_7 (Math|Vector|MakeVector (.x _origin) (.y _origin) _returnvalue_5))
  (bind _returnvalue_8 (- _returnvalue_3 _returnvalue_4))
  (bind _returnvalue_9 (Math|Vector|VectorLength _returnvalue_8))
  (bind _returnvalue_10 (* _returnvalue_6 _returnvalue_9))
  (|CallParentFunction)
  (bind _asbp_gamemode_0 (Utilities|Casting|CastToBP_Gamemode_0 (Game|GetGameMode)))
  (Default|StartBossFight _asbp_gamemode_0 "Insect Brood Mother")
  (Default|SetBossPercent _asbp_gamemode_0 (/ (Variables|Default|GetHealth) (Variables|Default|GetMax%20Health)))
  (Variables|Default|SetFight%20Started true)
  (Utilities|FlowControl|Delay 2.0)
  (Character|LaunchCharacter (Math|Vector|MakeVector (.x _returnvalue_10) (.y _returnvalue_10) 8e+02) false false)
  (Utilities|FlowControl|Delay 1.0)
  (Utilities|FlowControl|ForLoopwithBreak 0 500 :!label _label
    (:LoopBody
      (Utilities|FlowControl|Delay 0.2)
      (if (not (AI|Components|NavMovement|IsFalling (Variables|Character|GetCharacterMovement)))
        (goto _label Break)))
    (:Completed
      (Utilities|FlowControl|Delay 0.2)
      (Game|SpawnActorfromClass "/Game/Blueprints/NPC/Enemy/Brood_Mother_01/Phase_1/Hitboxes/BP_BroodMother_Slam_01.BP_BroodMother_Slam_01_C" (Math|Transform|MakeTransform _returnvalue_7 (.rotation _returnvalue_2) (.scale _returnvalue_2)) "Undefined" "MultiplyWithRoot" 0 3e+02 false 0)
      (Niagara|SpawnSystematLocation "/Game/Blueprints/NPC/Enemy/Brood_Mother_01/Phase_1/FX/NS_BroodMother_Slam.NS_BroodMother_Slam" _returnvalue_7)
      (CallFunction|CameraShake)
      (CallFunction|BootLegFacePlayer)
      (CallFunction|StartAttack))))

(event EventNextPhase
  (bind _outactors (Actor|GetAllActorsOfClass "/Game/Blueprints/World/BP_Location_Set.BP_Location_Set_C"))
  (for _array_element _outactors
    (if (== (Variables|/Game/Blueprints/World/BP_Location_Set.BP_Location_Set_C|GetPoint%20Number _array_element) 0)
      (Variables|Default|SetTarget%201 (Transformation|GetActorLocation _array_element))
      (elif (== (Variables|/Game/Blueprints/World/BP_Location_Set.BP_Location_Set_C|GetPoint%20Number _array_element) 1)
        (Variables|Default|SetTarget%202 (Transformation|GetActorLocation _array_element))
        (elif (== (Variables|/Game/Blueprints/World/BP_Location_Set.BP_Location_Set_C|GetPoint%20Number _array_element) 3)
          (Variables|Default|SetTarget%204 (Transformation|GetActorLocation _array_element))))))
  (if (Utilities|Operators|NotEqual(!=) :A (Variables|Default|GetTarget%202))
    (bind _returnvalue (Game|SpawnActorfromClass "/Game/Blueprints/NPC/Enemy/Brood_Mother_01/Phase_2/BP_Husk_Knight_01.BP_Husk_Knight_01_C" (Math|Transform|MakeTransform (Variables|Default|GetTarget%204) (Math|Rotator|FindLookatRotation (Variables|Default|GetTarget%202) (Variables|Default|GetTarget%201)) "1.000000,1.000000,1.000000") "Undefined" "MultiplyWithRoot" 0 0))
    (Default|StartBossFight _returnvalue)
    (bind _outactors_2 (Actor|GetAllActorsOfClass "/Game/Blueprints/NPC/Enemy/Spawner_01/BP_Spawner_01.BP_Spawner_01_C"))
    (for _array_element_2 _outactors_2
      (Utilities|IsValid _array_element_2
        (:Is%20Valid
          (Actor|DestroyActor))))
    (else
      (Actor|DestroyActor))))

(fn ConstructionScript
  (|CallParentFunction))