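; Master boss enemy Blueprint that handles taking damage, with empty StartBossFight and NextPhase events as hooks.
; Any damage triggers StartBossFight until FightStarted is set; hits from master hitboxes then spawn crit-aware damage numbers at the upper mesh bounds.
; Those hits reduce Health and send the health fraction to the game mode.
; At zero health, small bosses switch on mesh physics and multi-phase bosses call NextPhase.
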(event Custom|Start%20Boss%20Fight)

(event Custom|Next%20Phase)

(event EventBeginPlay)

(event Collision|EventActorBeginOverlap
  (params (OtherActor :type Actor%20Object%20Reference)))

(event EventTick
  (params (DeltaSeconds :type Float%20%28single-precision%29)))

(event Game|Damage|EventAnyDamage
  (params (Damage :type Float%20%28single-precision%29) (DamageType :type Damage%20Type%20Object%20Reference) (InstigatedBy :type Controller%20Object%20Reference) (DamageCauser :type Actor%20Object%20Reference))
  (if (not (Variables|Default|GetFight%20Started))
    (CallFunction|StartBossFight))
  (bind _asbp_master_hitbox_01 (Utilities|Casting|CastToBP_Master_Hitbox_01 DamageCauser))
  (bind _transform (CallFunction|GetBoundingBoxTop))
  (Game|SpawnActorfromClass "/Game/Blueprints/UI/BP_Damage_Number_01.BP_Damage_Number_01_C" _transform "Undefined" "MultiplyWithRoot" 0 (Utilities|String|ToString(Integer) (Math|Float|Truncate Damage)) (Variables|/Game/Blueprints/Hitbox/BP_Master_Hitbox_01.BP_Master_Hitbox_01_C|GetCrit _asbp_master_hitbox_01) 0)
  (bind _output_get (Variables|Default|SetHealth (- (Variables|Default|GetHealth) Damage)))
  (bind _asbp_gamemode_0 (Utilities|Casting|CastToBP_Gamemode_0 (Game|GetGameMode)))
  (Default|SetBossPercent _asbp_gamemode_0 (/ (Variables|Default|GetHealth) (Variables|Default|GetMax%20Health)))
  (if (<= _output_get 0.0)
    (if (< (Variables|Default|GetSize) 2)
      (Physics|SetSimulatePhysics (Variables|Character|GetMesh) true))
    (if (> (Variables|Default|GetPhases) 1)
      (CallFunction|NextPhase))))

(fn ConstructionScript)

(fn GetBoundingBoxTop
  (bind _mesh (Variables|Character|GetMesh))
  (bind _returnvalue (Physics|GetCenterOfMass _mesh "None"))
  (bind (_x _y _z) (Math|Vector|BreakVector _returnvalue))
  (return (Math|Transform|MakeTransform (Math|Vector|MakeVector _x _y (+ _z (/ (.Z (Math|Vector|BreakVector (.BoxExtent (Collision|GetComponentBounds _mesh)))) 2.0))))))