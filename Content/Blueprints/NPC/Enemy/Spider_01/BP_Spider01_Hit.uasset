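; BP_Spider01_Hit is a short-lived damage volume for Spider_01 attacks that destroys itself 0.2 seconds after spawning.
; Actors overlapping its box, other than the instigator, are recorded in HitActors so each is processed only once.
; When the instigator's controller is valid, each newly recorded actor takes DamageOfAbility damage, credited to that controller with the volume as causer.
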(event OnComponentBeginOverlap(Box)
  (params (OverlappedComponent :type Primitive%20Component%20Object%20Reference) (OtherActor :type Actor%20Object%20Reference) (OtherComp :type Primitive%20Component%20Object%20Reference) (OtherBodyIndex :type Integer) (bFromSweep :type Boolean) (SweepResult :type Hit%20Result%20Structure%20%28by%20ref%29))
  (bind _returnvalue (Game|GetInstigator))
  (bind _hit_actors (Variables|Default|GetHit%20Actors))
  (bind _returnvalue_2 (Pawn|GetController _returnvalue))
  (if (!= OtherActor (Game|GetInstigator))
    (if (not (Utilities|Array|ContainsItem _hit_actors OtherActor))
      (Utilities|Array|Add _hit_actors OtherActor)
      (Utilities|IsValid _returnvalue_2
        (:Is%20Valid
          (Game|Damage|ApplyDamage OtherActor (Variables|Default|GetDamage%20of%20Ability) _returnvalue_2 self))))))

(event EventBeginPlay
  (|CallParentFunction)
  (Utilities|FlowControl|Delay 0.2)
  (Actor|DestroyActor))

(event Collision|EventActorBeginOverlap
  (params (OtherActor :type Actor%20Object%20Reference))
  (|CallParentFunction OtherActor) ; This node is disabled and will not be called.\nDrag off pins to build functionality.
)

(event EventTick
  (params (DeltaSeconds :type Float%20%28single-precision%29))
  (|CallParentFunction DeltaSeconds) ; This node is disabled and will not be called.\nDrag off pins to build functionality.
)

(fn ConstructionScript
  (|CallParentFunction))