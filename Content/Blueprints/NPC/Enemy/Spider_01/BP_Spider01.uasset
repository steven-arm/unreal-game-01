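; BP_Spider01 is the "Insect Worker" spider enemy, which sets its health and named healthbar on spawn and attacks BP_Dawn in close range.
; Pawn sensing reveals the healthbar, sets a blackboard seen-enemy flag once, and triggers attacks.
; Taking damage also reveals the bar and briefly moves it toward the instigator.
; Attacks override the mesh animation, spawn a delayed hit actor, then restore the AnimBP under a DoOnce cooldown.
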(event OnSeePawn(PawnSensing)
  (params (Pawn :type Pawn%20Object%20Reference))
  (if (> (Variables|Default|GetHealth) 0.0)
    (bind _asbp_dawn (Utilities|Casting|CastToBP_Dawn Pawn))
    (Utilities|FlowControl|Sequence
      (:then_0
        (Utilities|FlowControl|DoOnce false
          (:Completed
            (Rendering|SetVisibility (Variables|Default|GetHealthbar) true false)
            (Variables|Default|SetHas%20Seen%20Enemy true)
            (AI|Components|Blackboard|SetValueasBool (AI|GetBlackboard (AI|GetAIController self)) (Utilities|Name|MakeLiteralName "Has Seen Enemy") true))))
      (:then_1
        (if (<= (Math|Vector|Distance(Vector) (Transformation|GetWorldLocation (Variables|/Script/Engine.Character|GetMesh _asbp_dawn)) (Transformation|GetWorldLocation (Variables|Default|GetCapsuleComponent))) 3e+02)
          (CallFunction|BasicAttack))))))

(event Custom|Basic%20Attack
  (bind _spawner (Variables|Default|GetSpawner))
  (bind _returnvalue (Transformation|GetWorldRotation _spawner))
  ;[1 1 1] Basic Attack
  (if (> (Variables|Default|GetHealth) 0.0)
    (Utilities|FlowControl|DoOnce false :!label _label
      (:Completed
        (Components|Animation|OverrideAnimationData (Variables|Character|GetMesh) "/Game/Blueprints/NPC/Enemy/Spider_01/Animation/AS_Spider_Attack_01.AS_Spider_Attack_01" false true 0.0 1.0)
        (Utilities|FlowControl|Delay 1.0)
        (Game|SpawnActorfromClass "/Game/Blueprints/NPC/Enemy/Spider_01/BP_Spider01_Hit.BP_Spider01_Hit_C" (Math|Transform|MakeTransform (Transformation|GetWorldLocation _spawner) (Math|Rotator|MakeRotator 0.0 (.pitch _returnvalue) (.yaw _returnvalue)) "1.000000,1.000000,1.000000") "Undefined" "MultiplyWithRoot" 0 25.0 false 0)
        (Components|Animation|SetAnimationMode (Variables|Character|GetMesh) "AnimationBlueprint" true)
        (Utilities|FlowControl|Delay 2.0)
        (goto _label Reset)))))

(event Custom|OnTakeAnyDamage_Event
  (params (DamagedActor :type Actor%20Object%20Reference) (Damage :type Float%20%28single-precision%29) (DamageType :type Damage%20Type%20Object%20Reference) (InstigatedBy :type Controller%20Object%20Reference) (DamageCauser :type Actor%20Object%20Reference))
  (bind _self self)
  (if (Variables|Default|GetHas%20Seen%20Enemy)
    _
    (else
      (Variables|Default|SetHas%20Seen%20Enemy true)
      (Rendering|SetVisibility (Variables|Default|GetHealthbar) true false)))
  (AI|AIMoveTo _self "0, 0, 0" InstigatedBy 5.0 false
    (:then
      (Utilities|FlowControl|Delay 1.0)
      (AI|Navigation|StopMovement (Pawn|GetController _self)))))

(event EventBeginPlay
  (|CallParentFunction)
  (Variables|Default|SetSize 1)
  (bind _output_get (Variables|Default|SetHealth 2e+02))
  (Variables|Default|SetMax%20Health _output_get)
  (bind _output_get_2 (Variables|Default|SetDisplay%20Name "Insect Worker"))
  (bind _aswbp_enemy_healthbar_01 (Utilities|Casting|CastToWBP_Enemy_Healthbar_01 (UserInterface|GetWidget (Variables|Default|GetHealthbar))))
  (Default|SetName _aswbp_enemy_healthbar_01 _output_get_2)
  (Default|SetPercent _aswbp_enemy_healthbar_01 1.0)
  (EventDispatchers|BindEventtoOnTakeAnyDamage (delegate Custom|OnTakeAnyDamage_Event)))

(event Collision|EventActorBeginOverlap
  (params (OtherActor :type Actor%20Object%20Reference))
  (|CallParentFunction OtherActor) ; This node is disabled and will not be called.\nDrag off pins to build functionality.
)

(event EventTick
  (params (DeltaSeconds :type Float%20%28single-precision%29))
  (|CallParentFunction DeltaSeconds) ; This node is disabled and will not be called.\nDrag off pins to build functionality.
)

(fn ConstructionScript
  (|CallParentFunction))